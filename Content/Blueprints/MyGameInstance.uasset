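; Game instance that owns the save game object and handles loading and saving it to a single named slot.
; On Init it loads the slot synchronously, or creates a fresh BP_SaveGame if none exists.
; Interface-style events offer sync or async load and save, plus a player-data write that saves immediately, and a getter exposes the cached object.
; Only a completed async load calls OnGameLoaded.
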(event EventInit
  (CallFunction|IFLoadGameData false))

(event EventIFSaveGameData
  (params (Async :type Boolean))
  ;[1 1 0 0.5] Save Game
  (if Async
    (|AsyncSaveGametoSlot (Variables|Default|GetSaveGameData) (Variables|Default|GetSlotName))
    (else
      (SaveGame|SaveGametoSlot (Variables|Default|GetSaveGameData) (Variables|Default|GetSlotName)))))

(event EventIFLoadGameData
  (params (Async :type Boolean))
  ;[1 1 0 0.5] Load Game
  (bind _returnvalue (SaveGame|DoesSaveGameExist (Variables|Default|GetSlotName)))
  (if _returnvalue
    (if Async
      (bind _savegame (|AsyncLoadGamefromSlot (Variables|Default|GetSlotName))
        (:Completed
          (bind _asbp_save_game (Utilities|Casting|CastToBP_SaveGame _savegame))
          (Variables|Default|SetSaveGameData _asbp_save_game)
          (Default|CallOnGameLoaded)))
      (else
        (bind _returnvalue_2 (SaveGame|LoadGamefromSlot (Variables|Default|GetSlotName)))
        (bind _asbp_save_game_2 (Utilities|Casting|CastToBP_SaveGame _returnvalue_2))
        (Variables|Default|SetSaveGameData _asbp_save_game_2)))
    (else
      (bind _returnvalue_3 (SaveGame|CreateSaveGameObject "/Game/Blueprints/SaveSystem/BP_SaveGame.BP_SaveGame_C"))
      (Variables|Default|SetSaveGameData _returnvalue_3))))

(event EventIFSavePlayer
  (params (PlayerSave :type S%20Player%20Saved%20Data%20Structure) (Async :type Boolean))
  (Variables|/Game/Blueprints/SaveSystem/BP_SaveGame.BP_SaveGame_C|SetPlayerSaveData (Variables|Default|GetSaveGameData) PlayerSave)
  (CallFunction|IFSaveGameData Async))

(fn IFGetGameData
  (return (Variables|Default|GetSaveGameData)))