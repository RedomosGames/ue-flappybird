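; Player character for a tap-to-bounce score game: the bounce input launches it upward while play is active.
; GS_Gameplay start and game-over events toggle gravity, input mode and the menu, gameplay and game-over widgets, with the camera attached to BP_CameraPos.
; Tagged overlaps end the game or add a point, debounced by a timed DoOnce.
; Per-difficulty high scores load and save through GameInstance interface messages.
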(event OnComponentBeginOverlap(BoxDetection)
  (params (OverlappedComponent :type Primitive%20Component%20Object%20Reference) (OtherActor :type Actor%20Object%20Reference) (OtherComp :type Primitive%20Component%20Object%20Reference) (OtherBodyIndex :type Integer) (bFromSweep :type Boolean) (SweepResult :type Hit%20Result%20Structure%20%28by%20ref%29))
  ;[1 1 0 0.5] Detect what player collides with
  (Utilities|FlowControl|Sequence
    (:then_0
      (if (Components|ComponentHasTag OtherComp "Bad")
        (CallFunction|CEGameOver)))
    (:then_1
      (if (Components|ComponentHasTag OtherComp "Score")
        (CallFunction|CEScorePoint)))))

(event Custom|CE_SetCameraPos
  (bind _returnvalue (Game|GetPlayerController 0))
  ;[1 1 0 0.5] Set Camera Position
  (Utilities|FlowControl|Sequence
    (:then_0
      (bind _returnvalue_2 (Actor|GetActorOfClass "/Game/Blueprints/GamePlay/BP_CameraPos.BP_CameraPos_C"))
      (Transformation|AttachComponentToComponent (Variables|Default|GetCamera) (Variables|/Game/Blueprints/GamePlay/BP_CameraPos.BP_CameraPos_C|GetArrow _returnvalue_2) "None" "KeepRelative" "KeepRelative" "KeepRelative" true))
    (:then_1
      (Input|SetInputModeUIOnly _returnvalue 0 "DoNotLock" false)
      (Variables|/Script/Engine.PlayerController|SetbShowMouseCursor _returnvalue true))))

(event Custom|CE_Widgets
  ;[0 0 1 0.5] Widgets
  (bind _returnvalue (UserInterface|CreateWidget "/Game/Blueprints/UI/WBP_MainMenu.WBP_MainMenu_C"))
  (bind _output_get (Variables|Widgets|SetMainMenuWidget _returnvalue))
  (UserInterface|Viewport|AddtoViewport _output_get 0)
  (bind _returnvalue_2 (UserInterface|CreateWidget "/Game/Blueprints/UI/WBP_GameOver.WBP_GameOver_C"))
  (bind _output_get_2 (Variables|Widgets|SetGameOverWIdget _returnvalue_2))
  (UserInterface|Viewport|AddtoViewport _output_get_2 0)
  (Widget|SetVisibility _output_get_2 "Collapsed")
  (bind _returnvalue_3 (UserInterface|CreateWidget "/Game/Blueprints/UI/WBP_GameplaySCreen.WBP_GameplaySCreen_C"))
  (bind _output_get_3 (Variables|Widgets|SetGameplayWidget _returnvalue_3))
  (UserInterface|Viewport|AddtoViewport _output_get_3 0)
  (Widget|SetVisibility _output_get_3 "Collapsed"))

(event Custom|CE_GameOver_Bind
  (bind _returnvalue (Game|GetPlayerController 0))
  ;[0.2 1 0 0.5] Bind Events
  (Variables|/Script/Engine.CharacterMovementComponent|SetGravityScale (Variables|Character|GetCharacterMovement) 0.0)
  (Variables|Default|SetIsPlaying? false)
  (Widget|SetVisibility (Variables|Widgets|GetGameOverWIdget) "Visible")
  (Input|SetInputModeUIOnly _returnvalue 0 "DoNotLock" false)
  (Variables|/Script/Engine.PlayerController|SetbShowMouseCursor _returnvalue true)
  (Widget|SetVisibility (Variables|Widgets|GetGameplayWidget) "Collapsed"))

(event Custom|CE_ScorePoint
  ;[1 1 0 0.5] Increase Player Score
  (Audio|PlaySound2D "/Engine/VREditor/Sounds/UI/Selection_Changes.Selection_Changes" 1.0 1.0 0.0 0 0)
  (Utilities|FlowControl|DoOnce false :!label _label
    (:Completed
      (CallFunction|FSetPlayerScore)
      (Utilities|FlowControl|Delay 1.5)
      (goto _label Reset))))

(event Custom|CE_Bindings
  ;[0.2 1 0 0.5] Bindings
  (EventDispatchers|BindEventtoOnGameStart (Variables|Cast|GetGameStateRef) (EventDispatchers|CreateEvent :!event Custom|CE_GameSart_Bind))
  (EventDispatchers|BindEventtoOnGameOver (Variables|Cast|GetGameStateRef) (EventDispatchers|CreateEvent :!event Custom|CE_GameOver_Bind)))

(event Custom|CE_GameSart_Bind
  (bind _returnvalue (Game|GetPlayerController 0))
  ;[0.2 1 0 0.5] Bind Events
  (Variables|/Script/Engine.CharacterMovementComponent|SetGravityScale (Variables|Character|GetCharacterMovement) 1.0)
  (Variables|Default|SetIsPlaying? true)
  (Widget|SetVisibility (Variables|Widgets|GetMainMenuWidget) "Collapsed")
  (Input|SetInputModeGameOnly _returnvalue false)
  (Variables|/Script/Engine.PlayerController|SetbShowMouseCursor _returnvalue false)
  (Widget|SetVisibility (Variables|Widgets|GetGameplayWidget) "Visible"))

(event Custom|CE_Casts
  ;[0 1 0.9946 0.5] Casts
  (bind _asgs_gameplay (Utilities|Casting|CastToGS_Gameplay (Game|GetGameState)))
  (Variables|Cast|SetGameStateRef _asgs_gameplay))

(event Custom|CE_GameOver
  ;[1 1 0 0.5] Call Game over
  (Audio|PlaySound2D "/Engine/VREditor/Sounds/UI/Invalid_Action.Invalid_Action" 1.0 1.0 0.0 0 0)
  (CallFunction|FSetPlayerHighScore)
  (Default|CallOnGameOver (Variables|Cast|GetGameStateRef))
  (bind _playersave (CallFunction|FGetSaveData))
  (Class|BPISaveGame|IFSavePlayer(Message) (Game|GetGameInstance) _playersave false))

(event Custom|CE_CheckHighScoreText
  (bind _mainmenuwidget (Variables|Widgets|GetMainMenuWidget))
  ;[1 1 0 0.5] Set High SCore Text
  (Rendering|Components|TextRender|SetText (Variables|/Game/Blueprints/UI/WBP_MainMenu.WBP_MainMenu_C|GetTXT_Easy_Score _mainmenuwidget) (Utilities|Text|ToText(Integer) (Variables|PlayStats|GetEasyHighSCore)))
  (Rendering|Components|TextRender|SetText (Variables|/Game/Blueprints/UI/WBP_MainMenu.WBP_MainMenu_C|GetTXT_Medium_Score _mainmenuwidget) (Utilities|Text|ToText(Integer) (Variables|PlayStats|GetMediumHighScore)))
  (Rendering|Components|TextRender|SetText (Variables|/Game/Blueprints/UI/WBP_MainMenu.WBP_MainMenu_C|GetTXT_Hard_Score _mainmenuwidget) (Utilities|Text|ToText(Integer) (Variables|PlayStats|GetHardHighSCore))))

(event Input|EnhancedActionEvents|EnhancedInputActionIA_Bounce
  (params (ActionValue :type Boolean) (ElapsedSeconds :type Float%20%28double-precision%29) (TriggeredSeconds :type Float%20%28double-precision%29) (InputAction :type Input%20Action%20Object%20Reference :default "/Game/Input/Actions/IA_Bounce.IA_Bounce"))
  ;[1 1 0 0.5] Launch Player When LMB is Pressed
  (:Started
    (Audio|PlaySound2D "/Engine/VREditor/Sounds/UI/Floating_UI_Close.Floating_UI_Close" 1.0 1.0 0.0 0 0)
    (if (Variables|Default|GetIsPlaying?)
      (Character|LaunchCharacter (Math|Vector|MakeVector 0.0 0.0 (Variables|Default|GetJumpForce)) false true))))

(event EventControllerChanged
  (params (OldController :type Controller%20Object%20Reference) (NewController :type Controller%20Object%20Reference))
  ;[1 0 0 0.5] Add Mapping Context
  (bind _asplayer_controller (Utilities|Casting|CastToPlayerController NewController))
  (Input|AddMappingContext (PlayerController|LocalPlayerSubsystems|GetEnhancedInputLocalPlayerSubsystem _asplayer_controller) "/Game/Input/IMC_Default.IMC_Default" 0 "(bIgnoreAllPressedKeysUntilRelease=True,bForceImmediately=False,bNotifyUserSettings=False)"))

(event EventPossessed
  (params (NewController :type Controller%20Object%20Reference))
  ;[1 0 0 0.5] Add Mapping Context
  (if (Class|Controller|IsPlayerController NewController)
    (bind _asplayer_controller (Utilities|Casting|CastToPlayerController NewController))
    (Input|AddMappingContext (PlayerController|LocalPlayerSubsystems|GetEnhancedInputLocalPlayerSubsystem _asplayer_controller) "/Game/Input/IMC_MouseLook.IMC_MouseLook" 0 "(bIgnoreAllPressedKeysUntilRelease=True,bForceImmediately=False,bNotifyUserSettings=False)")))

(event EventBeginPlay
  ;[1 1 0 0.5] Begin Play
  (Utilities|FlowControl|DelayUntilNextTick)
  (CallFunction|CECasts)
  (CallFunction|CEBindings)
  (CallFunction|CESetCameraPos)
  (CallFunction|CEWidgets)
  (bind _savegamedata (Class|BPISaveGame|IFGetGameData(Message) (Game|GetGameInstance)))
  (Utilities|IsValid _savegamedata
    (:Is%20Valid
      (CallFunction|FUsePlayerSave (Variables|/Game/Blueprints/SaveSystem/BP_SaveGame.BP_SaveGame_C|GetPlayerSaveData _savegamedata))
      (CallFunction|CECheckHighScoreText))))

(fn ConstructionScript)

(fn FSetPlayerHighScore
  (bind _playerstats (Variables|PlayStats|GetPlayerStats))
  (bind (_easyscore _mediumscore _hardscore) (Utilities|Struct|BreakS_PlayerStats _playerstats))
  (switch Utilities|FlowControl|Switch|SwitchonE_GameDifficulty (Variables|/Game/Blueprints/GS_Gameplay.GS_Gameplay_C|GetGameDifficulty (Variables|Cast|GetGameStateRef))
    (:NewEnumerator1
      (if (> _easyscore (Variables|PlayStats|GetEasyHighSCore))
        (bind _output_get (Variables|PlayStats|SetEasyHighSCore _easyscore)))
      (Rendering|Components|TextRender|SetText (Variables|/Game/Blueprints/UI/WBP_GameOver.WBP_GameOver_C|GetTXT_HighScore (Variables|Widgets|GetGameOverWIdget)) (Utilities|Text|ToText(Integer) _output_get)))
    (:NewEnumerator2
      (if (> _mediumscore (Variables|PlayStats|GetMediumHighScore))
        (bind _output_get_2 (Variables|PlayStats|SetMediumHighScore _mediumscore)))
      (Rendering|Components|TextRender|SetText (Variables|/Game/Blueprints/UI/WBP_GameOver.WBP_GameOver_C|GetTXT_HighScore (Variables|Widgets|GetGameOverWIdget)) (Utilities|Text|ToText(Integer) _output_get_2)))
    (:NewEnumerator3
      (if (> _hardscore (Variables|PlayStats|GetHardHighSCore))
        (bind _output_get_3 (Variables|PlayStats|SetHardHighSCore _hardscore)))
      (Rendering|Components|TextRender|SetText (Variables|/Game/Blueprints/UI/WBP_GameOver.WBP_GameOver_C|GetTXT_HighScore (Variables|Widgets|GetGameOverWIdget)) (Utilities|Text|ToText(Integer) _output_get_3))))
  (return))

(fn FSetPlayerScore
  (bind _playerstats (Variables|PlayStats|GetPlayerStats))
  (bind (_easyscore _mediumscore _hardscore) (Utilities|Struct|BreakS_PlayerStats _playerstats))
  (switch Utilities|FlowControl|Switch|SwitchonE_GameDifficulty (Variables|/Game/Blueprints/GS_Gameplay.GS_Gameplay_C|GetGameDifficulty (Variables|Cast|GetGameStateRef))
    (:NewEnumerator1
      (bind _result (Math|Integer|IncrementInt _easyscore)
        (:%20%20
          (Rendering|Components|TextRender|SetText (Variables|/Game/Blueprints/UI/WBP_GameplaySCreen.WBP_GameplaySCreen_C|GetTXT_Score (Variables|Widgets|GetGameplayWidget)) (Utilities|Text|ToText(Integer) _result))
          (Rendering|Components|TextRender|SetText (Variables|/Game/Blueprints/UI/WBP_GameOver.WBP_GameOver_C|GetTXT_PlayerSCore (Variables|Widgets|GetGameOverWIdget)) (Utilities|Text|ToText(Integer) _result)))))
    (:NewEnumerator2
      (bind _result_2 (Math|Integer|IncrementInt _mediumscore)
        (:%20%20
          (Rendering|Components|TextRender|SetText (Variables|/Game/Blueprints/UI/WBP_GameplaySCreen.WBP_GameplaySCreen_C|GetTXT_Score (Variables|Widgets|GetGameplayWidget)) (Utilities|Text|ToText(Integer) _result_2))
          (Rendering|Components|TextRender|SetText (Variables|/Game/Blueprints/UI/WBP_GameOver.WBP_GameOver_C|GetTXT_PlayerSCore (Variables|Widgets|GetGameOverWIdget)) (Utilities|Text|ToText(Integer) _result_2)))))
    (:NewEnumerator3
      (bind _result_3 (Math|Integer|IncrementInt _hardscore)
        (:%20%20
          (Rendering|Components|TextRender|SetText (Variables|/Game/Blueprints/UI/WBP_GameplaySCreen.WBP_GameplaySCreen_C|GetTXT_Score (Variables|Widgets|GetGameplayWidget)) (Utilities|Text|ToText(Integer) _result_3))
          (Rendering|Components|TextRender|SetText (Variables|/Game/Blueprints/UI/WBP_GameOver.WBP_GameOver_C|GetTXT_PlayerSCore (Variables|Widgets|GetGameOverWIdget)) (Utilities|Text|ToText(Integer) _result_3))))))
  (return))

(fn FGetSaveData
  (return (Utilities|Struct|MakeS_PlayerSavedData (Variables|PlayStats|GetEasyHighSCore) (Variables|PlayStats|GetMediumHighScore) (Variables|PlayStats|GetHardHighSCore))))

(fn FUsePlayerSave
  (params (PlayerSave :type S%20Player%20Saved%20Data%20Structure))
  (bind (_easyhighscore _mediumhighscore _hardhighscore) (Utilities|Struct|BreakS_PlayerSavedData PlayerSave))
  (if (not (== (Variables|PlayStats|GetEasyHighSCore) _easyhighscore))
    (Variables|PlayStats|SetEasyHighSCore _easyhighscore)
    (Variables|PlayStats|SetMediumHighScore _mediumhighscore)
    (Variables|PlayStats|SetHardHighSCore _hardhighscore)))