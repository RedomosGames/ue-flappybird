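; BP_PipeManager spawns pipe obstacles during gameplay, choosing an Easy, Medium or Hard pipe class from the game difficulty stored in GS_Gameplay.
; One tick after BeginPlay it caches the game state, binds to its events and starts a looping spawn timer, then immediately pauses it.
; The game start event unpauses the timer and game over pauses it.
; Each pipe appears at SpawnLocation X/Y with a random height.
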(event Custom|CE_SpawnPipe
  ;[1 1 0 0.5] Spawn Pipe Timer
  (bind _returnvalue (Utilities|Time|SetTimerbyEvent (delegate Custom|SpawnPipe) 2.0 true))
  (Variables|Default|SetSpawnPipeTimer _returnvalue))

(event Custom|CE_Casts
  ;[1 1 0 0.5] Get Cast Refs
  (bind _asgs_gameplay (Utilities|Casting|CastToGS_Gameplay (Game|GetGameState)))
  (Variables|Default|SetGameStateRef _asgs_gameplay))

(event Custom|PauseTimer
  ;[1 1 0 0.5] Bindings
  (Utilities|Time|PauseTimerbyHandle (Variables|Default|GetSpawnPipeTimer)))

(event Custom|SpawnPipe
  (bind _spawnlocation (Variables|Default|GetSpawnLocation))
  (bind _spawnlocation_2 (Variables|Default|GetSpawnLocation))
  (bind _spawnlocation_3 (Variables|Default|GetSpawnLocation))
  ;[1 1 0 0.5] Spawn Pipe Timer
  (switch Utilities|FlowControl|Switch|SwitchonE_GameDifficulty (Variables|/Game/Blueprints/GS_Gameplay.GS_Gameplay_C|GetGameDifficulty (Variables|Default|GetGameStateRef))
    (:NewEnumerator1
      (Game|SpawnActorfromClass "/Game/Blueprints/GamePlay/BP_Pipe_Easy.BP_Pipe_Easy_C" (Math|Transform|MakeTransform (Math|Vector|MakeVector (.x _spawnlocation_2) (.y _spawnlocation_2) (Math|Random|RandomFloatinRange 1e+01 3.3e+02)) "0, 0, 0" "1.000000,1.000000,1.000000") "Undefined" "MultiplyWithRoot" 0 0))
    (:NewEnumerator2
      (Game|SpawnActorfromClass "/Game/Blueprints/GamePlay/BP_Pipe_Medium.BP_Pipe_Medium_C" (Math|Transform|MakeTransform (Math|Vector|MakeVector (.x _spawnlocation_3) (.y _spawnlocation_3) (Math|Random|RandomFloatinRange 1e+01 3.3e+02)) "0, 0, 0" "1.000000,1.000000,1.000000") "Undefined" "MultiplyWithRoot" 0 0))
    (:NewEnumerator3
      (Game|SpawnActorfromClass "/Game/Blueprints/GamePlay/BP_Pipe_Hard.BP_Pipe_Hard_C" (Math|Transform|MakeTransform (Math|Vector|MakeVector (.x _spawnlocation) (.y _spawnlocation) (Math|Random|RandomFloatinRange 1e+01 3.3e+02)) "0, 0, 0" "1.000000,1.000000,1.000000") "Undefined" "MultiplyWithRoot" 0 0))))

(event Custom|CE_Bindings
  ;[1 1 0 0.5] Bindings
  (EventDispatchers|BindEventtoOnGameStart (Variables|Default|GetGameStateRef) (delegate Custom|SartTimer))
  (EventDispatchers|BindEventtoOnGameOver (Variables|Default|GetGameStateRef) (delegate Custom|PauseTimer)))

(event Custom|SartTimer
  ;[1 1 0 0.5] Bindings
  (Utilities|Time|UnpauseTimerbyHandle (Variables|Default|GetSpawnPipeTimer)))

(event EventBeginPlay
  ;[1 1 0 0.5] OnBegin
  (Utilities|FlowControl|DelayUntilNextTick)
  (CallFunction|CECasts)
  (CallFunction|CEBindings)
  (CallFunction|CESpawnPipe)
  (CallFunction|PauseTimer))

(fn ConstructionScript)