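; BP_Pipe_Medium is a pipe obstacle actor that scrolls toward negative X during gameplay and destroys itself past a fixed X limit.
; One tick after BeginPlay, it caches GS_Gameplay, binds to its game-over event and starts movement.
; A very short looping timer, rather than Tick, nudges the root by a fixed step.
; Game over pauses that timer, freezing the pipe in place.
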(event Custom|MovePipe
  (bind _defaultsceneroot (Variables|Default|GetDefaultSceneRoot))
  (bind _relativelocation (Variables|/Script/Engine.SceneComponent|GetRelativeLocation _defaultsceneroot))
  ;[1 1 0 0.5] Move Pipe Left Until it reaches target and get Destroyed
  (if (> (.x (Transformation|GetWorldLocation (Variables|Default|GetDefaultSceneRoot))) -5e+02)
    (Transformation|SetRelativeLocation _defaultsceneroot (Math|Vector|MakeVector (- (.x _relativelocation) 0.25) (.y _relativelocation) (.z _relativelocation)) false false)
    (else
      (Actor|DestroyActor))))

(event Custom|CE_Casts
  ;[1 1 0 0.5] Get Cast Refs
  (bind _asgs_gameplay (Utilities|Casting|CastToGS_Gameplay (Game|GetGameState)))
  (Variables|Default|SetGameStateRef _asgs_gameplay))

(event Custom|CE_MovePipe
  ;[1 1 0 0.5] Move Pipe Left Until it reaches target and get Destroyed
  (bind _returnvalue (Utilities|Time|SetTimerbyEvent (delegate Custom|MovePipe) 0.001 true))
  (Variables|Default|SetMovePipeTimer _returnvalue))

(event Custom|CE_Bindings
  ;[1 1 0 0.5] Bindings
  (EventDispatchers|BindEventtoOnGameOver (Variables|Default|GetGameStateRef) (delegate Custom|PauseTimer)))

(event Custom|PauseTimer
  ;[1 1 0 0.5] Bindings
  (Utilities|Time|PauseTimerbyHandle (Variables|Default|GetMovePipeTimer)))

(event EventBeginPlay
  ;[1 1 0 0.5] Begin play
  (Utilities|FlowControl|DelayUntilNextTick)
  (CallFunction|CECasts)
  (CallFunction|CEBindings)
  (CallFunction|CEMovePipe))

(fn ConstructionScript)