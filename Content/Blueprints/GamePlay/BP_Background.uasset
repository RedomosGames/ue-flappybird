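; BP_Background is a scrolling background actor that slides along negative X and loops back to its start.
; BeginPlay waits one tick, starts the movement and records the root's world location as SpawnLoc.
; A very fast looping timer, rather than Tick, nudges the root's relative X in small fixed steps.
; At the world X limit it teleports back to SpawnLoc, despite a comment saying it gets destroyed.
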(event Custom|MovePipe
  (bind _defaultsceneroot (Variables|Default|GetDefaultSceneRoot))
  (bind _relativelocation (Variables|/Script/Engine.SceneComponent|GetRelativeLocation _defaultsceneroot))
  ;[1 1 0 0.5] Move Pipe Left Until it reaches target and get Destroyed
  (if (> (.x (Transformation|GetWorldLocation (Variables|Default|GetDefaultSceneRoot))) -7.5e+03)
    (Transformation|SetRelativeLocation _defaultsceneroot (Math|Vector|MakeVector (- (.x _relativelocation) 0.1) (.y _relativelocation) (.z _relativelocation)) false false)
    (else
      (Transformation|SetWorldLocation (Variables|Default|GetDefaultSceneRoot) (Variables|Default|GetSpawnLoc) false false))))

(event Custom|CE_Move
  ;[1 1 0 0.5] Move Pipe Left Until it reaches target and get Destroyed
  (Utilities|Time|SetTimerbyEvent (delegate Custom|MovePipe) 0.001 true))

(event EventBeginPlay
  ;[1 1 0 0.5] Begin play
  (Utilities|FlowControl|DelayUntilNextTick)
  (CallFunction|CEMove)
  (Variables|Default|SetSpawnLoc (Transformation|GetWorldLocation (Variables|Default|GetDefaultSceneRoot))))

(fn ConstructionScript)